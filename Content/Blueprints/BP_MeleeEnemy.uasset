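; BP_MeleeEnemy is a melee enemy Blueprint that attacks, carries weapons and takes projectile hits, relying on functions defined outside this graph.
; On BeginPlay it calls AddWeapon over a randomly sized index range, so the weapon count varies per spawn.
; The Asdf event forwards a side flag to Attack.
; Overlapping actors that cast to Projectile call DamageEntity on the enemy, leaving damage handling to the projectile.
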(event `self.asdf`
  (params (leftside :type Boolean))
  ;[1 1 1] Enemy attack
  (`self.Attack` leftside))

(event `self.ReceiveBeginPlay`
  ;[1 1 1] Add weapon and health
  (for _index (range (+ (`KismetMathLibrary.RandomIntegerInRange` 1 2) 1))
    (`self.AddWeapon` _index)))

(event `self.ReceiveActorBeginOverlap`
  (params (OtherActor :type "Actor Object Reference"))
  ;[1 1 1] Projectile overlap event
  (bind _asprojectile (cast `/Game/Blueprints/Projectile` OtherActor))
  (`/Game/Blueprints/Projectile.DamageEntity` _asprojectile self))

(fn `UserConstructionScript`
  (`parent.UserConstructionScript`))