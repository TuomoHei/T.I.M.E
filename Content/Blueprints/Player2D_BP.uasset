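; 2D player Blueprint that moves horizontally by adding axis-driven velocity each tick and acts on touched enemies and items.
; AttackRange overlaps toggle CanDamage on enemies and CanPickup on items, gating touch actions by proximity.
; A touch triggers TimeManipulator and line-traces using the deprojected screen position.
; Damageable enemies are destroyed, after a Weapon attack if one is held; pickable items replace the current Weapon through the Pickup component.
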(event `Key|Touch1` :consume false
  (params (Key :type "Key Structure"))
  (bind _returnvalue (`GameplayStatics.GetPlayerController` 0))
  (bind (_locationx _locationy) (`PlayerController.GetInputTouchState` _returnvalue "Touch1"))
  (bind (_worldlocation _worlddirection) (`PlayerController.DeprojectScreenPositionToWorld` _returnvalue _locationx _locationy))
  ;[1 1 1] Line Trace To killEnemy
  (:`Pressed`
    (`KismetSystemLibrary.PrintString` "Faggot")
    (`TimeManipulator.Action` (`self.TimeManipulator`))
    (bind _outhit (`KismetSystemLibrary.LineTraceSingle` (0.0 0.0 0.0) (+ (* _worldlocation 3000.0) _worlddirection) "TraceTypeQuery1"))
    (bind _output_get (set `self.HitActor` (`.HitActor` (`GameplayStatics.BreakHitResult` _outhit))))
    (bind _asbp_enemy_2d (cast `/Game/Blueprints/BP_Enemy2D` _output_get)
      (:`then`
        ;[1 1 1] Attack
        (if (`/Game/Blueprints/BP_Enemy2D.bCanDamage` _asbp_enemy_2d)
          (`/Engine/EditorBlueprintResources/StandardMacros.IsValid` (`self.Weapon`)
            (:`Is Valid`
              (bind _asweapon_bp (cast `/Game/Blueprints/Weapon_BP` (`self.Weapon`)))
              (`/Game/Blueprints/Weapon_BP.Attack` _asweapon_bp))
            (:`Is Not Valid`
              _))
          (`self.K2_DestroyActor` _asbp_enemy_2d)))
      (:`CastFailed`
        (bind _asbp_item_2 (cast `/Game/Blueprints/BP_Item2` _output_get))
        ;[1 1 1] PickUp
        (if (`/Game/Blueprints/BP_Item2.bCanPickup` _asbp_item_2)
          (`/Engine/EditorBlueprintResources/StandardMacros.IsValid` (`self.Weapon`)
            (:`Is Valid`
              (`PickupComponent.DisEquip` (`self.Pickup`) (`self.Weapon`)))
            (:`Is Not Valid`
              _))
          (bind _output_get_2 (set `self.Weapon` _asbp_item_2))
          (`PickupComponent.Pickup` (`self.Pickup`) _output_get_2)
          (set `/Game/Blueprints/BP_Item2.bCanPickup` false _output_get_2))))))

(event `self.ReceiveBeginPlay`
  ;[1 1 1] Initializeing Player
  (`PickupComponent.SetPlayer` (`self.Pickup`) self)
  (`self.EnableInput` (`GameplayStatics.GetPlayerController` 0))
  (set `PlayerController.bShowMouseCursor` true (`GameplayStatics.GetPlayerController` 0)))

(event `self.ReceiveTick`
  (params (DeltaSeconds :type "Float (single-precision)"))
  ;[1 1 1] Move to Mouse Pos
  (`self.K2_SetActorLocation` (+ (`self.K2_GetActorLocation`) (`self.Velocity`))))

(event `InputAxis|MoveRight`
  (params (AxisValue :type "Float (single-precision)"))
  ;[1 1 1] Move to Mouse Pos
  (set `self.Velocity` (`KismetMathLibrary.MakeVector` (* AxisValue 2.0))))

(event `self.AttackRange.OnComponentBeginOverlap`
  (params (OverlappedComponent :type "PrimitiveComponent Object Reference") (OtherActor :type "Actor Object Reference") (OtherComp :type "PrimitiveComponent Object Reference") (OtherBodyIndex :type Integer) (bFromSweep :type Boolean) (SweepResult :type "HitResult Structure (by ref)"))
  ;[1 1 1] Collision To Enemy
  (bind _asbp_enemy_2d (cast `/Game/Blueprints/BP_Enemy2D` OtherActor)
    (:`then`
      (set `/Game/Blueprints/BP_Enemy2D.bCanDamage` true _asbp_enemy_2d))
    (:`CastFailed`
      ;[1 1 1] Collision To Item
      (bind _asbp_item_2 (cast `/Game/Blueprints/BP_Item2` OtherActor))
      (set `/Game/Blueprints/BP_Item2.bCanPickup` true _asbp_item_2))))

(event `self.AttackRange.OnComponentEndOverlap`
  (params (OverlappedComponent :type "PrimitiveComponent Object Reference") (OtherActor :type "Actor Object Reference") (OtherComp :type "PrimitiveComponent Object Reference") (OtherBodyIndex :type Integer))
  ;[1 1 1] Collision To Enemy
  (bind _asbp_enemy_2d (cast `/Game/Blueprints/BP_Enemy2D` OtherActor)
    (:`then`
      (set `/Game/Blueprints/BP_Enemy2D.bCanDamage` false _asbp_enemy_2d))
    (:`CastFailed`
      ;[1 1 1] Collision To Item
      (bind _asbp_item_2 (cast `/Game/Blueprints/BP_Item2` OtherActor))
      (set `/Game/Blueprints/BP_Item2.bCanPickup` false _asbp_item_2))))

(fn `UserConstructionScript`)