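; Side-scroller orthographic camera actor that takes over the player's view at BeginPlay and follows the player pawn.
; Each Tick it interpolates toward the pawn plus a horizontal offset chosen by control yaw, then forces a fixed rotation.
; Follow speed scales with horizontal distance to that target, clamped between minimum and maximum.
; It also eases ortho width between normal and slowed zoom according to the level's TimeManager slow state.
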(event `self.ReceiveBeginPlay`
  ;[1 1 1] Init camera settings
  (`CameraComponent.SetProjectionMode` (`self.CameraComponent`) "Orthographic") ; Make sure projection mode is se to Orthographic
  (`PlayerController.SetViewTargetWithBlend` (`GameplayStatics.GetPlayerController` 0) self 0.0 "VTBlend_Linear" 0.0 false)
  ;[1 1 1] Get reference to Time Manager
  (bind _outactors (`GameplayStatics.GetAllActorsOfClass` "/Script/CppTest.TimeManager"))
  (for _array_element _outactors
    (set `self.TimeManager` _array_element)))

(event `self.ReceiveTick`
  (params (DeltaSeconds :type "Float (single-precision)"))
  (bind _returnvalue (`GameplayStatics.GetPlayerPawn` 0))
  (bind _cameracomponent (`self.CameraComponent`))
  (bind _cameratargetoffsetx (`self.CameraTargetOffsetX`))
  (bind _returnvalue_2 (`KismetMathLibrary.MakeTransform` (`KismetMathLibrary.MakeVector` (+ (.x (.location (`self.GetTransform` _returnvalue))) (`KismetMathLibrary.SelectFloat` (* _cameratargetoffsetx -1.0) _cameratargetoffsetx (> (.yaw (`Pawn.GetControlRotation` _returnvalue)) 0.0))) (.y (.location (`self.GetTransform` _returnvalue))) (.z (.location (`self.GetTransform` _returnvalue))))))
  ;[1 1 1] Camera Movement
  (`/Engine/EditorBlueprintResources/StandardMacros.IsValid` _returnvalue
    (:`Is Valid`
      (bind _returnvalue_3 (`TimeManager.GetSlow` (`self.TimeManager`)))
      (`CameraComponent.SetOrthoWidth` _cameracomponent (`KismetMathLibrary.FInterpTo` (`CameraComponent.OrthoWidth` _cameracomponent) (`KismetMathLibrary.SelectFloat` (`self.SlowedZoom`) (`self.NormalZoom`) _returnvalue_3) DeltaSeconds (`self.ZoomSpeed`)))
      (bind _lerpspeed (`self.CalculateLerpSpeed` _returnvalue_2 (.x (.location (`self.GetTransform`)))))
      (`self.K2_SetActorTransform` (`KismetMathLibrary.TInterpTo` (`KismetMathLibrary.MakeTransform` (+ (`KismetMathLibrary.MakeVector` (.x (.location (`self.GetTransform`))) (.y (.location (`self.GetTransform`))) (.z (.location (`self.GetTransform`)))) (`self.CameraOffset`))) _returnvalue_2 DeltaSeconds _lerpspeed)) ; Set Camera Position
      (`self.K2_SetActorRotation` (struct :`Yaw` -90.0)))))

(fn `CalculateLerpSpeed`
  (params (TargetTransform :type "Transform Structure") (CameraX :type "Float (double-precision)"))
  (returns (LerpSpeed :type "Float (double-precision)"))
  (locals (isCamLeftOfPlayer :type Boolean :default false))
  (return (`KismetMathLibrary.FClamp` (* (`KismetMathLibrary.Abs` (- (.x (.location TargetTransform)) CameraX)) (`self.SmoothMultiplier`)) (`self.MinCamSpeed`) (`self.MaxCamSpeed`))))

(fn `UserConstructionScript`)