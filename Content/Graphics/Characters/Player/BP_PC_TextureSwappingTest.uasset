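; Test Blueprint for runtime texture swapping on the player character mesh, toggled by pressing P.
; On BeginPlay it creates a dynamic instance of M_PlayerCharacter, assigns it to the mesh's first material slot and enables input.
; Each P press runs a FlipFlop that alternates that instance between two player textures.
; The texture parameter names are all None, so the calls target no named material parameter.
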(event `self.ReceiveBeginPlay`
  (bind _mesh_playercharacter (`self.Mesh_PlayerCharacter`))
  (bind _returnvalue (`PrimitiveComponent.CreateDynamicMaterialInstance` _mesh_playercharacter 0 "/Game/Graphics/Characters/Player/M_PlayerCharacter.M_PlayerCharacter" "None"))
  (`PrimitiveComponent.SetMaterial` _mesh_playercharacter 0 _returnvalue)
  (`self.EnableInput` (`GameplayStatics.GetPlayerController` 0)))

(event `Key|P`
  (params (Key :type "Key Structure"))
  (:`Pressed`
    (`/Engine/EditorBlueprintResources/StandardMacros.FlipFlop`
      (:`A`
        (`MaterialInstanceDynamic.SetTextureParameterValue` (stale `self.ReceiveBeginPlay` _returnvalue) "None" "/Game/Graphics/Characters/Player/T_PlayerCharacter_01.T_PlayerCharacter_01")
        (`MaterialInstanceDynamic.SetTextureParameterValue` (stale `self.ReceiveBeginPlay` _returnvalue) "None" "/Game/Graphics/Characters/Player/T_PlayerCharacter_01.T_PlayerCharacter_01"))
      (:`B`
        (`MaterialInstanceDynamic.SetTextureParameterValue` (stale `self.ReceiveBeginPlay` _returnvalue) "None" "/Game/Graphics/Characters/Player/T_PlayerCharacter_02.T_PlayerCharacter_02")
        (`MaterialInstanceDynamic.SetTextureParameterValue` (stale `self.ReceiveBeginPlay` _returnvalue) "None" "/Game/Graphics/Characters/Player/T_PlayerCharacter_02.T_PlayerCharacter_02")))))

(fn `UserConstructionScript`)