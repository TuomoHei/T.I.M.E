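; BP_Train is an animated background train that periodically runs along negative X and then resets.
; BeginPlay stores the start location, disables ticking and sets a looping timer with a random 30 to 45 second interval, rolled once, to re-enable it.
; While active, Tick moves the train by speed and delta time until it has travelled 10000 units, then snaps it back and switches ticking off.
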(event `ActivateTrain`
  ;[1 1 1] ActivateTrain (enable ticking)
  (`self.SetActorTickEnabled` true))

(event `self.ReceiveBeginPlay`
  ;[1 1 1] BeginPlay (set a timer to activate train)
  (`KismetSystemLibrary.K2_SetTimer` null "ActivateTrain" (`KismetMathLibrary.RandomFloatInRange` 30.0 45.0) true) ; Set a timer to activate train in intervals
  (set `self.InitialLocation` (`self.K2_GetActorLocation`))
  (`self.SetActorTickEnabled` false))

(event `self.ReceiveTick`
  (params (DeltaSeconds :type "Float (single-precision)"))
  ;[1 1 1] Tick (If train is activated, move it until it has traveled a certain distance)
  (if (< (- (.x (`self.InitialLocation`)) (.x (`self.K2_GetActorLocation`))) 10000.0)
    (`self.K2_SetActorLocation` (+ (`self.K2_GetActorLocation`) (`KismetMathLibrary.MakeVector` (* (* (`self.Speed`) -1.0) (`GameplayStatics.GetWorldDeltaSeconds`)))))
    (else
      (`self.K2_SetActorLocation` (`self.InitialLocation`))
      (`self.SetActorTickEnabled` false))))

(fn `UserConstructionScript`)