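; Weapon_BP is a 2D projectile weapon item that runs item physics while unattached and fires when held by an Enemy2D.
; UseWeapon reads the holder's Direction and calls Attack, gated by a fire-rate cooldown that Tick counts down.
; Attack spawns a projectile at the sprite's transform, passes it the direction, and spends Endurance, detaching and destroying the weapon when it runs out.
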(event `self.ReceiveTick`
  (params (DeltaSeconds :type "Float (single-precision)"))
  ;[1 1 1] Counter for shoottime
  (bind _output_get (set `self.shoottime` (- (`self.shoottime`) DeltaSeconds)))
  ;[1 1 1] Item physics and pickup
  (`/Engine/EditorBlueprintResources/StandardMacros.IsValid` (`self.GetAttachParentActor`)
    (:`Is Not Valid`
      (`self.Physics` DeltaSeconds))))

(event `self.UseWeapon`
  ;[1 1 1] Get the direction of user and shoot
  (bind _asenemy_2d (cast `Enemy2D` (`self.GetAttachParentActor`)))
  (if (< (stale `self.ReceiveTick` _output_get) 0.0)
    (`self.Attack` (`Enemy2D.direction` _asenemy_2d))
    (set `self.shoottime` (`self.firerate`))))

(fn `Attack`
  (params (direction :type "Vector Structure"))
  ;[1 1 1] Spawning actor and setting direction
  (bind _returnvalue (`|SpawnActorFromClass` "/Game/Blueprints/Projectile.Projectile_C" (`SceneComponent.K2_GetComponentToWorld` (`self.PaperSprite`)) "Undefined" "OverrideRootScale" null (0.0 0.0 0.0) null))
  (set `/Game/Blueprints/Projectile.direction` direction _returnvalue)
  ;[1 1 1] Endurance counter
  (bind _output_get (set `self.endurance` (- (`self.endurance`) 1)))
  (if (<= _output_get 0)
    (`self.K2_DetachFromActor` "KeepWorld" "KeepWorld" "KeepWorld")
    (`self.K2_DestroyActor`)
    (else
      (`KismetSystemLibrary.PrintString` "Endurance" (`KismetMathLibrary.Conv_IntToBool` _output_get)))))

(fn `UserConstructionScript`
  (`parent.UserConstructionScript`))