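; Camera actor that smoothly follows the first player's pawn at a fixed orientation.
; Each Tick, while the pawn is valid, it interpolates from its own location plus WorldOffset toward the pawn's transform, then overrides the rotation with a constant.
; Because the offset feeds the interpolation's current value rather than its target, the trailing distance depends on frame time as well as WorldOffset.
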(event `self.ReceiveTick`
  (params (DeltaSeconds :type "Float (single-precision)"))
  (bind _returnvalue (`GameplayStatics.GetPlayerPawn` 0))
  ;[1 1 1] Camera Movement
  (`/Engine/EditorBlueprintResources/StandardMacros.IsValid` _returnvalue
    (:`Is Valid`
      (`self.K2_SetActorTransform` (`KismetMathLibrary.TInterpTo` (`KismetMathLibrary.MakeTransform` (+ (`KismetMathLibrary.MakeVector` (.x (.location (`self.GetTransform`))) (.y (.location (`self.GetTransform`))) (.z (.location (`self.GetTransform`)))) (`self.WorldOffset`))) (`self.GetTransform` _returnvalue) DeltaSeconds 3.0))
      (`self.K2_SetActorRotation` (struct :`Yaw` -90.0)))))

(fn `UserConstructionScript`)