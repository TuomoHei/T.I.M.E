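; Base-style 2D weapon item that falls under physics when loose and can be used by the Player2D it is attached to.
; Tick calls Physics only while the item has no attached parent actor.
; UseWeapon calls UnEquip on the owning Player2D once Endurance is zero or below, otherwise it calls Shoot.
; Shoot is an empty event here, and this graph never decrements Endurance.
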(event `self.ReceiveTick`
  (params (DeltaSeconds :type "Float (single-precision)"))
  ;[1 1 1] Item physics and pickup
  (`/Engine/EditorBlueprintResources/StandardMacros.IsValid` (`self.GetAttachParentActor`)
    (:`Is Not Valid`
      (`self.Physics` DeltaSeconds))))

(event `self.UseWeapon`
  ;[1 1 1] Endurance check
  (if (<= (`self.endurance`) 0)
    (bind _asplayer_2d (cast `Player2D` (`self.GetAttachParentActor`)))
    (`Player2D.UnEquip` _asplayer_2d)
    (else
      (`self.Shoot`))))

(event `Shoot`)

(fn `UserConstructionScript`)