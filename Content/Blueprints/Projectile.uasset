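; A 2D projectile actor that flies horizontally and damages either the player or enemies, then destroys itself after a set lifetime or on a successful hit.
; Tick moves it without sweep along the X component of its normalized Direction, scaled by Speed and delta time.
; DamageEntity uses BoolEnemy to choose between killing a Player2D and damaging an Enemy2D, with debug prints.
; No collision event in this file calls DamageEntity.
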(event `self.ReceiveBeginPlay`
  ;[1 1 1] Check if the component spawned is attached
  (`KismetSystemLibrary.Delay` (`self.LifeTime`))
  (`self.K2_DestroyActor`))

(event `self.ReceiveTick`
  (params (DeltaSeconds :type "Float (single-precision)"))
  ;[1 1 1] Projectile movement
  (`self.K2_SetActorLocation` (+ (`self.K2_GetActorLocation`) (* (`KismetMathLibrary.MakeVector` (.x (`KismetMathLibrary.Normal` (`self.direction`)))) (* DeltaSeconds (`self.speed`))))))

(fn `DamageEntity`
  (params (Entity :type "Actor Object Reference"))
  ;[1 1 1] Called when projectile hits
  (if (`self.Bool enemy`)
    (bind _asplayer_2d (cast `Player2D` Entity))
    (`Player2D.PlayerDeath` _asplayer_2d)
    (`self.K2_DestroyActor`)
    (`KismetSystemLibrary.PrintString` "Playerd")
    (else
      (bind _asenemy_2d (cast `Enemy2D` Entity))
      (`Enemy2D.TakeDamageEnemy` _asenemy_2d true)
      (`self.K2_DestroyActor`)
      (`KismetSystemLibrary.PrintString` "EnemyD"))))

(fn `UserConstructionScript`)