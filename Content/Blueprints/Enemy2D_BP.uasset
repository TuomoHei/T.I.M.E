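; 2D enemy that chases the player horizontally and destroys them on contact.
; BeginPlay caches the first Player2D_BP found, and Tick moves the enemy along X toward it at fixed speed with unswept SetActorLocation.
; A Hit event destroys the player if it is the hit actor.
; Gravity and IsGrounded are set but never read in these graphs, so movement is horizontal only.
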(event `self.ReceiveHit`
  (params (MyComp :type "PrimitiveComponent Object Reference") (Other :type "Actor Object Reference") (OtherComp :type "PrimitiveComponent Object Reference") (bSelfMoved :type Boolean) (HitLocation :type "Vector Structure") (HitNormal :type "Vector Structure") (NormalImpulse :type "Vector Structure") (Hit :type "HitResult Structure (by ref)"))
  (bind _playerref (`self.PlayerRef`))
  ;[1 1 1] Kill Player
  (set `self.bIsGrounded` true)
  (if (and (`self.bIsPlayerValid`) (== (`.HitActor` (`GameplayStatics.BreakHitResult` Hit)) _playerref))
    (`self.K2_DestroyActor` _playerref)
    (`KismetSystemLibrary.PrintString` "Killed Player!")))

(event `self.ReceiveBeginPlay`
  ;[1 1 1] Initialize Enemy
  (`ActorComponent.SetAutoActivate` (`self.Slow`) true)
  (set `self.Gravity` 2.0)
  (bind _outactors (`GameplayStatics.GetAllActorsOfClass` "/Game/Blueprints/Player2D_BP.Player2D_BP_C"))
  (if (> (`KismetArrayLibrary.Array_Length` _outactors) 0)
    (set `self.PlayerRef` (`|GetArrayItem` _outactors))))

(event `self.ReceiveTick`
  (params (DeltaSeconds :type "Float (single-precision)"))
  (bind _playerref (`self.PlayerRef`))
  (set `self.DeltaTime` DeltaSeconds)
  ;[1 1 1] CalcVelocityFromPlayerPosition
  (bind _output_get (set `self.bIsPlayerValid` (`KismetSystemLibrary.IsValid` _playerref)))
  (if _output_get
    (set `self.CurrentPos` (`self.K2_GetActorLocation`))
    (if (>= (.x (`self.K2_GetActorLocation` _playerref)) (.x (`self.CurrentPos`)))
      (set `self.VelocityX` 100.0)
      (else
        (set `self.VelocityX` -100.0)))
    ;[1 1 1] Move
    (`self.K2_SetActorLocation` (+ (`KismetMathLibrary.MakeVector` (* (`self.VelocityX`) (`self.DeltaTime`))) (`self.CurrentPos`)))))

(fn `UserConstructionScript`)