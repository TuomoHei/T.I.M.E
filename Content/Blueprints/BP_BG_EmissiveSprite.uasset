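; Background emissive sprite Blueprint that animates the opacity of its static mesh's material.
; BeginPlay creates a dynamic material instance and picks a random phase offset.
; Each Tick, EffectIndex selects a sine wave or flicker effect, whose value drives the Opacity parameter.
; The sine uses speed and offset, while Flicker ignores the offset and lerps on time modulo speed, giving a repeating ramp.
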(event `self.ReceiveBeginPlay`
  (bind _staticmeshcomponent (`self.StaticMeshComponent`))
  (bind _returnvalue (`PrimitiveComponent.CreateDynamicMaterialInstance` _staticmeshcomponent 0 (`PrimitiveComponent.GetMaterial` _staticmeshcomponent 0) "None"))
  (`PrimitiveComponent.SetMaterial` _staticmeshcomponent 0 _returnvalue)
  (set `self.DynamicMaterial` _returnvalue)
  (set `self.RandomOffset` (`KismetMathLibrary.RandomFloatInRange` 0.0 50.0)))

(event `self.ReceiveTick`
  (params (DeltaSeconds :type "Float (single-precision)"))
  (bind _returnvalue (`KismetSystemLibrary.GetGameTimeInSeconds`))
  (bind _speed (`self.Speed`))
  (bind _minvalue (`self.MinValue`))
  (bind _maxvalue (`self.MaxValue`))
  (bind _randomoffset (`self.RandomOffset`))
  (bind _dynamicmaterial (`self.DynamicMaterial`))
  (switch `int` (`self.EffectIndex`)
    (:`0`
      (bind _returnvalue_2 (`self.Sinewave` _returnvalue _minvalue _maxvalue _speed _randomoffset))
      (set `self.EffectTempFloat` _returnvalue_2))
    (:`1`
      (bind _returnvalue_3 (`self.Flicker` _returnvalue _minvalue _maxvalue _speed _randomoffset))
      (set `self.EffectTempFloat` _returnvalue_3)))
  (`MaterialInstanceDynamic.SetScalarParameterValue` _dynamicmaterial "Opacity" (`self.EffectTempFloat`))
  (`PrimitiveComponent.SetMaterial` (`self.StaticMeshComponent`) 0 _dynamicmaterial))

(fn `Flicker`
  (params (Time :type "Float (double-precision)") (MinValue :type "Float (double-precision)") (MaxValue :type "Float (double-precision)") (Speed :type "Float (double-precision)") (Offset :type "Float (double-precision)"))
  (returns (ReturnValue :type "Float (double-precision)"))
  (return (`KismetMathLibrary.Lerp` MinValue MaxValue (mod Time Speed))))

(fn `Sinewave`
  (params (Time :type "Float (double-precision)") (MinValue :type "Float (double-precision)") (MaxValue :type "Float (double-precision)") (Speed :type "Float (double-precision)") (Offset :type "Float (double-precision)"))
  (returns (ReturnValue :type "Float (double-precision)"))
  (return (`KismetMathLibrary.Lerp` MinValue MaxValue (* (+ (`KismetMathLibrary.DegSin` (+ (* Time Speed) Offset)) 1.0) 0.5))))

(fn `UserConstructionScript`)