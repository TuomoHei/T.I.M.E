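; BP_SceneScoreActor is an in-scene score display that shows the score multiplier as a number with a timer-driven ring.
; On BeginPlay it creates a dynamic material instance for its static mesh and stores it.
; Each Tick it derives the material's Alpha parameter linearly from MultiplierTimer to update the ring.
; It also writes ScoreMultiplier to the MultiplierNumber text, leaving it blank unless the multiplier exceeds one.
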(event `self.ReceiveBeginPlay`
  (bind _staticmesh (`self.StaticMesh`))
  (bind _returnvalue (`PrimitiveComponent.CreateDynamicMaterialInstance` _staticmesh 0 (`PrimitiveComponent.GetMaterial` _staticmesh 0) "None"))
  (`MaterialInstanceDynamic.SetScalarParameterValue` _returnvalue "Alpha" 1.0)
  (`PrimitiveComponent.SetMaterial` _staticmesh 0 _returnvalue)
  (set `self.DynamicMaterial` _returnvalue))

(event `self.ReceiveTick`
  (params (DeltaSeconds :type "Float (single-precision)"))
  (bind _dynamicmaterial (`self.DynamicMaterial`))
  (bind _multipliernumber (`self.MultiplierNumber`))
  (bind _scoremultiplier (`self.ScoreMultiplier`))
  (`MaterialInstanceDynamic.SetScalarParameterValue` _dynamicmaterial "Alpha" (- 1.0 (* (`self.MultiplierTimer`) 0.2)))
  (`PrimitiveComponent.SetMaterial` (`self.StaticMesh`) 0 _dynamicmaterial)
  (if (> _scoremultiplier 1)
    (`TextRenderComponent.K2_SetText` _multipliernumber (`KismetTextLibrary.Conv_IntToText` _scoremultiplier))
    (else
      (`TextRenderComponent.K2_SetText` _multipliernumber (`KismetTextLibrary.Conv_StringToText` "")))))

(fn `UserConstructionScript`)