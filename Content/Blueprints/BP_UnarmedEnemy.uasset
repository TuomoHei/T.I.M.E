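; Unarmed enemy Blueprint that attacks with left or right hit volumes and takes damage from projectiles.
; Attack picks a side, and OnAttack briefly shows that side's AttackRange and enables its collision after a short delay.
; Overlapping actors that cast to Projectile call DamageEntity on the enemy and print a debug string.
; CalcVelocity and SetAttackState are empty, with only disconnected logic left inside.
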(event `self.asdf`
  (params (leftside :type Boolean))
  ;[1 1 1] Enemy Attack
  (`self.Attack` leftside))

(event `self.ReceiveActorBeginOverlap`
  (params (OtherActor :type "Actor Object Reference"))
  ;[1 1 1] Projectile hit event
  (`self.HitFunc` OtherActor))

(event `OnAttack`
  (params (LorR :type String))
  (switch `string` LorR
    (:`Default`
      (`KismetSystemLibrary.Delay` 0.2 :!label _label)
      (`SceneComponent.SetVisibility` (`self.AttackRangeL`) true false)
      (`PrimitiveComponent.SetCollisionEnabled` (`self.AttackRangeL`) "QueryAndPhysics")
      (`KismetSystemLibrary.Delay` 0.2)
      (`SceneComponent.SetVisibility` (`self.AttackRangeL`) false false)
      (`PrimitiveComponent.SetCollisionEnabled` (`self.AttackRangeL`) "NoCollision"))
    (:`Right`
      (`KismetSystemLibrary.Delay` 0.2)
      (`SceneComponent.SetVisibility` (`self.AttackRangeR`) true false)
      (`PrimitiveComponent.SetCollisionEnabled` (`self.AttackRangeR`) "QueryAndPhysics")
      (`KismetSystemLibrary.Delay` 0.2)
      (`SceneComponent.SetVisibility` (`self.AttackRangeR`) false false)
      (`PrimitiveComponent.SetCollisionEnabled` (`self.AttackRangeR`) "NoCollision"))
    (:`Left`
      (goto _label)))
  (`self.SetAttackState`))

(fn `Attack`
  (params (BLaam :type Boolean))
  (if BLaam
    (`self.OnAttack` "Right")
    (else
      (`self.OnAttack` "Left")))
  (`SceneComponent.K2_AddWorldRotation` (`self.AttackRangeL`) (struct :`Pitch` 1.0) false false)
  (`SceneComponent.K2_AddWorldRotation` (`self.AttackRangeR`) (struct :`Pitch` 1.0) false false))

(fn `CalcVelocity`
  (params (Target :type "Actor Object Reference"))
  (returns (ReturnValue :type "Vector Structure")))

(fn `HitFunc`
  (params (BulletObject :type "Actor Object Reference"))
  (bind _asprojectile (cast `/Game/Blueprints/Projectile` BulletObject))
  (`/Game/Blueprints/Projectile.DamageEntity` _asprojectile self)
  (`KismetSystemLibrary.PrintString` "Hello"))

(fn `SetAttackState`)

(fn `UserConstructionScript`)