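; BP_ParallaxBackground is a background mesh that scrolls its material for a parallax effect.
; On BeginPlay it creates a dynamic material instance with configurable U and V tiling.
; Each tick it sets U, and V when Y scrolling is enabled, from GetActiveCameraPosition scaled by ScrollSpeed.
; That function's graph shows only an unconnected camera-location lookup, with no wired return value.
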(event `self.ReceiveBeginPlay`
  (bind _staticmeshcomponent (`self.StaticMeshComponent`))
  (bind _returnvalue (`PrimitiveComponent.CreateDynamicMaterialInstance` _staticmeshcomponent 0 (`PrimitiveComponent.GetMaterial` _staticmeshcomponent 0) "None"))
  (`MaterialInstanceDynamic.SetScalarParameterValue` _returnvalue "UTiling" (`self.UTiling`))
  (`MaterialInstanceDynamic.SetScalarParameterValue` _returnvalue "VTiling" (`self.VTiling`))
  (`PrimitiveComponent.SetMaterial` _staticmeshcomponent 0 _returnvalue)
  (set `self.DynamicMaterial` _returnvalue))

(event `self.ReceiveTick`
  (params (DeltaSeconds :type "Float (single-precision)"))
  (bind _dynamicmaterial (`self.DynamicMaterial`))
  (bind _scrollspeed (`self.ScrollSpeed`))
  (`MaterialInstanceDynamic.SetScalarParameterValue` _dynamicmaterial "U" (* (.x (`PlayerCameraManager.GetCameraLocation` (`GameplayStatics.GetPlayerCameraManager` 0))) _scrollspeed))
  (if (`self.EnableYScrolling`)
    (`MaterialInstanceDynamic.SetScalarParameterValue` _dynamicmaterial "V" (* (.y (`PlayerCameraManager.GetCameraLocation` (`GameplayStatics.GetPlayerCameraManager` 0))) _scrollspeed)))
  (`PrimitiveComponent.SetMaterial` (`self.StaticMeshComponent`) 0 _dynamicmaterial))

(fn `UserConstructionScript`)