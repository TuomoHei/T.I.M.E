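; Animated background sprite actor that pulses the opacity of its static mesh material over time.
; BeginPlay creates a dynamic material instance from the mesh's first material slot.
; Each Tick turns game time and a Speed variable into a 0–1 degree-based sine wave, writes it to the Opacity parameter, and reassigns the material to the mesh.
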(event `self.ReceiveBeginPlay`
  (bind _staticmeshcomponent (`self.StaticMeshComponent`))
  (bind _returnvalue (`PrimitiveComponent.CreateDynamicMaterialInstance` _staticmeshcomponent 0 (`PrimitiveComponent.GetMaterial` _staticmeshcomponent 0) "None"))
  (`PrimitiveComponent.SetMaterial` _staticmeshcomponent 0 _returnvalue)
  (set `self.DynamicMaterial` _returnvalue))

(event `self.ReceiveTick`
  (params (DeltaSeconds :type "Float (single-precision)"))
  (bind _dynamicmaterial (`self.DynamicMaterial`))
  (bind _returnvalue (`self.Sinewave` (`KismetSystemLibrary.GetGameTimeInSeconds`) (`self.Speed`)))
  (`MaterialInstanceDynamic.SetScalarParameterValue` _dynamicmaterial "Opacity" _returnvalue)
  (`PrimitiveComponent.SetMaterial` (`self.StaticMeshComponent`) 0 _dynamicmaterial))

(fn `Sinewave`
  (params (Time :type "Float (double-precision)") (Speed :type "Float (double-precision)"))
  (returns (ReturnValue :type "Float (double-precision)"))
  (return (* (+ (`KismetMathLibrary.DegSin` (* Time Speed)) 1.0) 0.5)))

(fn `UserConstructionScript`)