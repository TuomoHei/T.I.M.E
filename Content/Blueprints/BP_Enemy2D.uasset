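; 2D enemy that chases the first Player2D_BP along X, destroys it on hit, and calls DropItem when destroyed.
; Tick moves it at fixed speed without sweep until SetAttackState finds the player close on X, then fires OnAttack toward that side while rotating both attack ranges.
; OnAttack waits a cooldown, briefly enables that side's range visibility and collision, then rechecks range, relying on Delays to absorb per-tick calls.
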(event `self.ReceiveHit`
  (params (MyComp :type "PrimitiveComponent Object Reference") (Other :type "Actor Object Reference") (OtherComp :type "PrimitiveComponent Object Reference") (bSelfMoved :type Boolean) (HitLocation :type "Vector Structure") (HitNormal :type "Vector Structure") (NormalImpulse :type "Vector Structure") (Hit :type "HitResult Structure (by ref)"))
  (bind _playerref (`self.PlayerRef`))
  ;[1 1 1] Kill Player
  (if (and (`self.bIsPlayerValid`) (== (`.HitActor` (`GameplayStatics.BreakHitResult` Hit)) _playerref))
    (`self.K2_DestroyActor` _playerref)
    (`KismetSystemLibrary.PrintString` "Killed Player!")))

(event `self.ReceiveBeginPlay`
  ;[1 1 1] Initialize Enemy
  (add `self.OnDestroyed` (delegate `DestroyEvent`))
  (bind _outactors (`GameplayStatics.GetAllActorsOfClass` "/Game/Blueprints/Player2D_BP.Player2D_BP_C"))
  (if (> (`KismetArrayLibrary.Array_Length` _outactors) 0)
    (set `self.PlayerRef` (`|GetArrayItem` _outactors))))

(event `DestroyEvent` :!signature `self.OnDestroyed`
  (params (DestroyedActor :type "Actor Object Reference"))
  (`self.Drop` (`self.DropItem`)))

(event `self.ReceiveTick`
  (params (DeltaSeconds :type "Float (single-precision)"))
  (bind _playerref (`self.PlayerRef`))
  (set `self.DeltaTime` DeltaSeconds)
  (bind _output_get (set `self.bIsPlayerValid` (`KismetSystemLibrary.IsValid` _playerref)))
  (if _output_get
    (bind _returnvalue (`self.CalcVelocity` _playerref))
    (if (`self.bCanAttack`)
      (if (<= (`self.Distance`) 0.0)
        (`self.OnAttack` "Right")
        (else
          (`self.OnAttack` "Left")))
      (`SceneComponent.K2_AddWorldRotation` (`self.AttackRangeL`) (struct :`Pitch` 1.0) false false)
      (`SceneComponent.K2_AddWorldRotation` (`self.AttackRangeR`) (struct :`Pitch` 1.0) false false)
      (else
        ;[1 1 1] Move
        (`self.K2_SetActorLocation` _returnvalue)
        (`self.SetAttackState`)))))

(event `OnAttack`
  (params (LorR :type String))
  (switch `string` LorR
    (:`Default`
      (`KismetSystemLibrary.Delay` (`self.CoolTime`) :!label _label)
      (`SceneComponent.SetVisibility` (`self.AttackRangeL`) true false)
      (`PrimitiveComponent.SetCollisionEnabled` (`self.AttackRangeL`) "QueryAndPhysics")
      (`KismetSystemLibrary.Delay` (`self.AttackTime`))
      (`SceneComponent.SetVisibility` (`self.AttackRangeL`) false false)
      (`PrimitiveComponent.SetCollisionEnabled` (`self.AttackRangeL`) "NoCollision"))
    (:`Right`
      (`KismetSystemLibrary.Delay` (`self.CoolTime`))
      (`SceneComponent.SetVisibility` (`self.AttackRangeR`) true false)
      (`PrimitiveComponent.SetCollisionEnabled` (`self.AttackRangeR`) "QueryAndPhysics")
      (`KismetSystemLibrary.Delay` (`self.AttackTime`))
      (`SceneComponent.SetVisibility` (`self.AttackRangeR`) false false)
      (`PrimitiveComponent.SetCollisionEnabled` (`self.AttackRangeR`) "NoCollision"))
    (:`Left`
      (goto _label)))
  (`self.SetAttackState`))

(fn `CalcVelocity`
  (params (Target :type "Actor Object Reference"))
  (returns (ReturnValue :type "Vector Structure"))
  ;[1 1 1] CalcVelocityFromPlayerPosition
  (set `self.PlayerPos` (`self.K2_GetActorLocation` Target))
  (set `self.CurrentPos` (`self.K2_GetActorLocation`))
  (if (>= (.x (`self.PlayerPos`)) (.x (`self.CurrentPos`)))
    (set `self.VelocityX` 100.0)
    (else
      (set `self.VelocityX` -100.0)))
  (return (+ (`KismetMathLibrary.MakeVector` (* (`self.VelocityX`) (`self.DeltaTime`))) (`self.CurrentPos`))))

(fn `SetAttackState`
  (bind _output_get (set `self.Distance` (- (.x (`self.CurrentPos`)) (.x (`self.PlayerPos`)))))
  (bind _returnvalue (<= (`KismetMathLibrary.Abs` _output_get) 70.0))
  (if _returnvalue
    _
    (else
      _))
  (set `self.bCanAttack` _returnvalue)
  (return))

(fn `UserConstructionScript`)